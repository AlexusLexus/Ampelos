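; Damage-over-time ability that repeatedly hurts the player referenced by PlayerRef, then ends itself.
; Tick paces the hits through a half-second Delay, sending a fixed DamageHealthMessage and incrementing Count after each wait.
; Once Count reaches MaxTick, Tick calls EndAbility.
; PlayerRef is not assigned in these graphs, and BeginPlay and overlap events do no work.
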(event `self.ReceiveTick`
  (params (DeltaSeconds :type "Float (single-precision)"))
  (if (< (`self.Count`) (`self.Max Tick`))
    (`KismetSystemLibrary.Delay` 0.5)
    (message `/Game/GameplayAbiltities/BPI_AbilitySystem.Damage Health` (`self.Player Ref`) 10.0)
    (`/Engine/EditorBlueprintResources/StandardMacros.IncrementInt` (`self.Count`))
    (else
      (`self.End Ability`))))

(fn `UserConstructionScript`
  (`parent.UserConstructionScript`))