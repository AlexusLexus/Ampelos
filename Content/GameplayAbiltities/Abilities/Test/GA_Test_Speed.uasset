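; Test gameplay ability that grants the player a speed bonus for as long as the ability exists.
; On ability start, a DoOnce gate adds SpeedValue to the player's AdditionalSpeed, so repeated starts do not stack it.
; When destroyed, it subtracts the same variable without checking whether the bonus was applied.
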(event `self.OnAbilityStart`
  (bind _player_ref (`self.Player Ref`))
  (`/Engine/EditorBlueprintResources/StandardMacros.DoOnce` false
    (:`Completed`
      (set `/Game/Character/Player/FirstPersonCharacter.Additional Speed` (+ (`/Game/Character/Player/FirstPersonCharacter.Additional Speed` _player_ref) (`self.Speed Value`)) _player_ref))))

(event `self.ReceiveDestroyed`
  (bind _player_ref (`self.Player Ref`))
  (set `/Game/Character/Player/FirstPersonCharacter.Additional Speed` (- (`/Game/Character/Player/FirstPersonCharacter.Additional Speed` _player_ref) (`self.Speed Value`)) _player_ref))

(fn `UserConstructionScript`
  (`parent.UserConstructionScript`))