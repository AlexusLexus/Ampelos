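; Prototype test quest that moves through two stages and prints a debug message for each.
; BeginPlay advances an unstarted quest to stage 5, and a player-tagged actor overlapping the 5To10 box sets stage 10.
; Both call QuestUpdate, which switches on the stage and prints behind a DoOnce per stage.
; The construction script pins the trigger box to a hardcoded world location and extent.
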(event `self.ReceiveBeginPlay`
  (if (== (`self.GetStage`) 0)
    (`self.AdvanceStage` 5)
    (`self.QuestUpdate`)))

(event `self.QuestUpdate`
  (switch `string` (`KismetStringLibrary.Conv_IntToString` (`self.Stage`))
    (:`5`
      ;[1 1 1] Stage 5
      (`/Engine/EditorBlueprintResources/StandardMacros.DoOnce` false
        (:`Completed`
          (`KismetSystemLibrary.PrintString` "Test Quest Stage 5" true true (struct :`G` 0.66 :`B` 1.0 :`A` 1.0) 5.0))))
    (:`10`
      ;[1 1 1] Stage 10
      (`/Engine/EditorBlueprintResources/StandardMacros.DoOnce` false
        (:`Completed`
          (`KismetSystemLibrary.PrintString` "Test Quest Stage 10" true true (struct :`G` 0.66 :`B` 1.0 :`A` 1.0) 5.0))))))

(event `self.5 to 10.OnComponentBeginOverlap`
  (params (OverlappedComponent :type "PrimitiveComponent Object Reference") (OtherActor :type "Actor Object Reference") (OtherComp :type "PrimitiveComponent Object Reference") (OtherBodyIndex :type Integer) (bFromSweep :type Boolean) (SweepResult :type "HitResult Structure (by ref)"))
  (if (`self.ActorHasTag` OtherActor "Ampelos.Player")
    (`self.SetStage` 10)
    (`self.QuestUpdate`)))

(fn `UserConstructionScript`
  (bind _5_to_10 (`self.5 to 10`))
  (`SceneComponent.K2_SetWorldLocation` _5_to_10 (-17051.5 10208.311523 2546.847412) false false)
  (`BoxComponent.SetBoxExtent` _5_to_10 (256.0 256.0 256.0) true))