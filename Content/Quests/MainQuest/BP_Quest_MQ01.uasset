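; BP_Quest_MQ01 is the first main quest's stage logic, carrying it from start to the player reaching the Old Town entrance.
; QuestUpdate switches on the current stage and advances stage 0 to 5 once.
; A hit on the entrance box by the player-tagged actor during stage 5 sets stage 10 once and re-runs QuestUpdate, which has no stage 10 case.
; The construction script hardcodes that box's world position and extent.
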(event `self.QuestUpdate`
  (switch `string` (`KismetStringLibrary.Conv_IntToString` (`self.GetStage`))
    (:`0`
      ;[1 1 1] Stage 0 (empty)
      (`/Engine/EditorBlueprintResources/StandardMacros.DoOnce` false
        (:`Completed`
          (`self.SetStage` 5)
          (`self.CallUpdate`))))))

(event `self.Stage 5 Old Town Entrance.OnComponentHit`
  (params (HitComponent :type "PrimitiveComponent Object Reference") (OtherActor :type "Actor Object Reference") (OtherComp :type "PrimitiveComponent Object Reference") (NormalImpulse :type "Vector Structure") (Hit :type "HitResult Structure (by ref)"))
  (if (and (`self.ActorHasTag` OtherActor "Ampelos.Player") (== (`self.GetStage`) 5))
    (`/Engine/EditorBlueprintResources/StandardMacros.DoOnce` false
      (:`Completed`
        (`self.SetStage` 10)
        (`self.QuestUpdate`)))))

(fn `UserConstructionScript`
  (bind _stage_5_old_town_entrance (`self.Stage 5 Old Town Entrance`))
  (`SceneComponent.K2_SetWorldLocation` _stage_5_old_town_entrance (-7905.0 7489.0 3300.0) false false)
  (`BoxComponent.SetBoxExtent` _stage_5_old_town_entrance (200.0 1000.0 256.0) true))