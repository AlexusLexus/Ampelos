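; Test vehicle that the player's FirstPersonCharacter mounts by pressing F, with no proximity check.
; The first press attaches the capsule to the Seat socket, disables its collision and activates a camera; the next restores collision and moves it to a hard-coded location, without detaching.
; MoveForward offsets the static mesh through a Timeline acceleration value and MoveRight yaws it.
; Once attached, Tick locks player capsule and camera yaw to the mesh.
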(event `self.ReceiveBeginPlay`
  (bind _asfirst_person_character (cast `/Game/Character/Player/FirstPersonCharacter` (`GameplayStatics.GetPlayerPawn` 0)))
  (set `self.Player Ref` _asfirst_person_character))

(event `Key|F`
  (params (Key :type "Key Structure"))
  (bind _player_ref (`self.Player Ref`))
  (bind _springarm (`/Game/Character/Player/FirstPersonCharacter.SpringArm` _player_ref))
  (bind _capsulecomponent (`Character.CapsuleComponent` _player_ref))
  (:`Pressed`
    (`/Engine/EditorBlueprintResources/StandardMacros.FlipFlop`
      (:`A`
        (`SceneComponent.K2_SetRelativeLocation` _capsulecomponent (0.0 0.0 100.0) false false)
        (`SceneComponent.K2_AttachToComponent` _capsulecomponent (`self.SkeletalMesh`) "Seat" "KeepRelative" "KeepRelative" "KeepRelative" true)
        (`PrimitiveComponent.SetCollisionEnabled` (`Character.CapsuleComponent` _player_ref) "NoCollision")
        (set `SpringArmComponent.TargetArmLength` 0.0 _springarm)
        (set `self.bAttached` true)
        (`ActorComponent.SetActive` (`self.Camera`) true false))
      (:`B`
        (`PrimitiveComponent.SetCollisionEnabled` (`Character.CapsuleComponent` _player_ref) "QueryAndPhysics")
        (`SceneComponent.K2_SetWorldLocation` _capsulecomponent (-16546.0 10502.0 2645.0) false false)
        (set `SpringArmComponent.TargetArmLength` 0.0 _springarm)))))

(event `self.ReceiveTick`
  (params (DeltaSeconds :type "Float (single-precision)"))
  (bind (_returnvalue_roll _returnvalue_pitch _returnvalue_yaw) (`KismetMathLibrary.BreakRotator` (`SceneComponent.K2_GetComponentRotation` (`self.StaticMesh`))))
  (if (`self.bAttached`)
    (`SceneComponent.K2_SetWorldRotation` (`Character.CapsuleComponent` (`self.Player Ref`)) (`KismetMathLibrary.MakeRotator` 0.0 0.0 (- _returnvalue_yaw 90.0)) false false)
    (`SceneComponent.K2_SetWorldRotation` (`/Game/Character/Player/FirstPersonCharacter.FirstPersonCamera` (`self.Player Ref`)) (`KismetMathLibrary.MakeRotator` 0.0 0.0 (- _returnvalue_yaw 90.0)) false false)))

(event `InputAxis|MoveForward` :consume false :overrideparent false
  (params (AxisValue :type "Float (single-precision)"))
  (`|ExecutionSequence`
    (:`then_0`
      (bind (_direction _acc) (`Timeline|Timeline_0`)))
    (:`then_1`
      (`SceneComponent.K2_AddWorldOffset` (`self.StaticMesh`) (* (`SceneComponent.GetForwardVector` (`self.DefaultSceneRoot`)) (* (* _acc AxisValue) 2.5)) false false))))

(event `InputAxis|MoveRight`
  (params (AxisValue :type "Float (single-precision)"))
  (`SceneComponent.K2_AddWorldRotation` (`self.DefaultSceneRoot`) (`KismetMathLibrary.MakeRotator` 0.0 0.0 (* AxisValue 0.18)) false false)
  (`SceneComponent.K2_AddWorldRotation` (`self.StaticMesh`) (`KismetMathLibrary.MakeRotator` 0.0 0.0 (* AxisValue 0.18)) false false))

(fn `UserConstructionScript`)